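; TriggerBox is a trigger actor that shows a message when the main character overlaps it.
; On BeginPlay it caches the first BP_MainCharacter found in the level.
; An overlap by that character copies TextToShow into Text and outputs it with PrintString.
; An overlap by any other actor, or any end overlap, clears Text and prints the empty string.
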(event EventBeginPlay
  (bind _outactors (Actor|GetAllActorsOfClass "/Game/GGJ2020Project/MainCharacter/BP_MainCharacter.BP_MainCharacter_C"))
  (Variables|Default|SetMainCharacter (Utilities|Array|Get(acopy) _outactors)))

(event Collision|EventActorBeginOverlap
  (params (OtherActor :type Actor%20Object%20Reference))
  (bind _maincharacter (Variables|Default|GetMainCharacter))
  (Utilities|IsValid _maincharacter
    (:Is%20Valid
      (if (== OtherActor _maincharacter)
        (bind _output_get (Variables|Default|SetText (Variables|Default|GetTextToShow)))
        (Development|PrintString _output_get)
        (else
          (bind _output_get_2 (Variables|Default|SetText ""))
          (Development|PrintString _output_get_2))))))

(event Collision|EventActorEndOverlap
  (params (OtherActor :type Actor%20Object%20Reference))
  (bind _output_get (Variables|Default|SetText ""))
  (Development|PrintString _output_get))

(fn ConstructionScript)