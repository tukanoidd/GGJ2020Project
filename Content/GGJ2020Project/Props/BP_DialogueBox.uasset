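; BP_DialogueBox is a prop that shows its TextToShow as subtitle text while the main character overlaps it.
; On BeginPlay it caches the first BP_MainCharacter found in the level.
; When that character begins overlapping, it writes TextToShow into the character's SubtitleText.
; Any end overlap clears that text, without checking which actor left.
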(event EventBeginPlay
  (bind _outactors (Actor|GetAllActorsOfClass "/Game/GGJ2020Project/MainCharacter/BP_MainCharacter.BP_MainCharacter_C"))
  (Variables|Default|SetMainCharacter (Utilities|Array|Get(acopy) _outactors)))

(event Collision|EventActorBeginOverlap
  (params (OtherActor :type Actor%20Object%20Reference))
  (bind _maincharacter (Variables|Default|GetMainCharacter))
  (Utilities|IsValid _maincharacter
    (:Is%20Valid
      (if (== OtherActor _maincharacter)
        (Variables|/Script/GGJ2020Project.MainCharacter|SetSubtitleText _maincharacter (Variables|Default|GetTextToShow))))))

(event Collision|EventActorEndOverlap
  (params (OtherActor :type Actor%20Object%20Reference))
  (Variables|/Script/GGJ2020Project.MainCharacter|SetSubtitleText (Variables|Default|GetMainCharacter) ""))

(fn ConstructionScript)